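; BP_PickupSprite is a world pickup that puts an item into the player's inventory when BP_Dude overlaps its sphere.
; The overlap calls AddItem on the character's inventory with the pickup's item class and amount.
; On partial success it keeps the leftover amount, otherwise it destroys itself.
; Either way, a successful pickup records its ID and remaining amount in the inventory's LootedPickup map.
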(event `self.Sphere.OnComponentBeginOverlap`
  (params (OverlappedComponent :type "PrimitiveComponent Object Reference") (OtherActor :type "Actor Object Reference") (OtherComp :type "PrimitiveComponent Object Reference") (OtherBodyIndex :type Integer) (bFromSweep :type Boolean) (SweepResult :type "HitResult Structure (by ref)"))
  (bind _asbp_dude (cast `/Game/DEMO/Blueprint/BP_Dude` OtherActor))
  (bind _inventoryref (`/Game/DEMO/Blueprint/BP_Dude.InventoryRef` _asbp_dude))
  (`/Engine/EditorBlueprintResources/StandardMacros.IsValid` _inventoryref
    (:`Is Valid`
      (bind (_success _rest) (`/Game/InventorySystem/blueprints/BP_Inventory.AddItem` _inventoryref (`self.itemToAdd`) (`self.amount`)))
      (if _success
        (if (> _rest 0)
          (set `self.amount` _rest)
          (bind _inventoryref_2 (`/Game/DEMO/Blueprint/BP_Dude.InventoryRef` _asbp_dude))
          (`KismetArrayLibrary.Array_Add` (`/Game/InventorySystem/blueprints/BP_Inventory.LootedPickup` _inventoryref_2) (make `/Game/InventorySystem/blueprints/structures/S_SavedPickup` (`self.ID`) (`self.amount`)))
          (else
            (`KismetArrayLibrary.Array_Add` (`/Game/InventorySystem/blueprints/BP_Inventory.LootedPickup` _inventoryref_2) (make `/Game/InventorySystem/blueprints/structures/S_SavedPickup` (`self.ID`)))
            (`self.K2_DestroyActor`)))))))

(fn `UserConstructionScript`)